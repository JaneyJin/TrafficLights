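; Traffic light Blueprint that shows its current red, yellow or green state on three separate light components.
; OnTrafficLightStateChanged switches on the incoming state and swaps material slot 1 on each component, giving the active light its lit streetlight material and the other two a shared off material.
; The Blueprint only handles the visual response, with no timing or state-cycling logic and an empty construction script.
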(event `self.OnTrafficLightStateChanged`
  (params (TrafficLightState :type "ETrafficLightState Enum" :default "Red"))
  (switch `ETrafficLightState` TrafficLightState
    (:`Red`
      (`PrimitiveComponent.SetMaterial` (`self.RedLight`) 1 "/Game/TrafficLightSign/MI_Streetlights_2.MI_Streetlights_2")
      (`PrimitiveComponent.SetMaterial` (`self.YellowLight`) 1 "/Game/TrafficLightSign/MI_StreetLightsOff.MI_StreetLightsOff")
      (`PrimitiveComponent.SetMaterial` (`self.GreenLight`) 1 "/Game/TrafficLightSign/MI_StreetLightsOff.MI_StreetLightsOff"))
    (:`Yellow`
      (`PrimitiveComponent.SetMaterial` (`self.RedLight`) 1 "/Game/TrafficLightSign/MI_StreetLightsOff.MI_StreetLightsOff")
      (`PrimitiveComponent.SetMaterial` (`self.YellowLight`) 1 "/Game/TrafficLightSign/MI_Streetlights_1.MI_Streetlights_1")
      (`PrimitiveComponent.SetMaterial` (`self.GreenLight`) 1 "/Game/TrafficLightSign/MI_StreetLightsOff.MI_StreetLightsOff"))
    (:`Green`
      (`PrimitiveComponent.SetMaterial` (`self.RedLight`) 1 "/Game/TrafficLightSign/MI_StreetLightsOff.MI_StreetLightsOff")
      (`PrimitiveComponent.SetMaterial` (`self.YellowLight`) 1 "/Game/TrafficLightSign/MI_StreetLightsOff.MI_StreetLightsOff")
      (`PrimitiveComponent.SetMaterial` (`self.GreenLight`) 1 "/Game/TrafficLightSign/MI_Streetlights_3.MI_Streetlights_3"))))

(fn `UserConstructionScript`)